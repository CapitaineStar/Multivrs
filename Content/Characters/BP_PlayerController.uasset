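; Player controller that possesses the assigned player and blends the view between it and a far camera framing given bounds.
; SwitchToFarCam spawns or reuses a BP_FarCam_Pawn, configures it with bounds and source location, then blends to it.
; SwitchToPlayer aligns control yaw to the far camera's spring arm, blends back and resets a timer.
; Tick runs that timer past the blend time before destroying the unused far camera.
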(event EventTick
  (params (DeltaSeconds :type Float%20%28single-precision%29))
  (if (< (Variables|Default|GetDestroyTimer) (Variables|Default|GetCameraBlendTime))
    (Variables|Default|SetDestroyTimer (+ (Variables|Default|GetDestroyTimer) DeltaSeconds))
    (elif (not (Variables|Default|GetIsUsingFarCamera))
      (bind _farcamref (Variables|Default|GetFarCamRef)
        (:then
          (Actor|DestroyActor _farcamref))
        (:else)))))

(fn ConstructionScript)

(fn SwitchtoFarCam
  (params (CameraBounds :type Sphere%20Component%20Object%20Reference) (SourceLocation :type Vector))
  (LocalVariables|Set_CamBounds CameraBounds)
  (LocalVariables|Set_SourceLocation SourceLocation)
  (Utilities|FlowControl|Sequence
    (:then_0
      (Utilities|IsValid (Variables|Default|GetFarCamRef)
        (:Is%20Not%20Valid
          (bind _returnvalue (Game|SpawnActorfromClass "/Game/Characters/FarCam/BP_FarCam_Pawn.BP_FarCam_Pawn_C" (Math|Conversions|ToTransform(Vector) (Transformation|GetWorldLocation (LocalVariables|Get_CamBounds))) "Undefined" 0 0))
          (Variables|Default|SetFarCamRef _returnvalue))))
    (:then_1
      (Default|SetupFarCamera (Variables|Default|GetFarCamRef) (LocalVariables|Get_CamBounds) (LocalVariables|Get_SourceLocation))
      (Game|Player|SetViewTargetwithBlend (Variables|Default|GetFarCamRef) (Variables|Default|GetCameraBlendTime) "VTBlend_Cubic" 0.0 false)
      (Variables|Default|SetIsUsingFarCamera true))))

(fn SwitchtoPlayer
  (Pawn|SetControlRotation (Math|Rotator|MakeRotator 0.0 -1e+01 (.Yaw (Math|Rotator|BreakRotator (Transformation|GetWorldRotation (Variables|/Game/Characters/FarCam/BP_FarCam_Pawn.BP_FarCam_Pawn_C|GetSpringArm (Variables|Default|GetFarCamRef)))))))
  (Game|Player|SetViewTargetwithBlend (Variables|Default|GetPlayerRef) (Variables|Default|GetCameraBlendTime) "VTBlend_Cubic" 0.0 false)
  (Variables|Default|SetIsUsingFarCamera false)
  (Variables|Default|SetDestroyTimer -1.0))

(fn AssignPlayer
  (params (PlayerRef :type BP%20Player%20Object%20Reference))
  (bind _output_get (Variables|Default|SetPlayerRef PlayerRef))
  (Pawn|Possess _output_get))