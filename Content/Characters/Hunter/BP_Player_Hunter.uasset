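; BP_Player_Hunter is the player-controlled Hunter character, handling movement and jump input.
; Forward and right axes apply movement while movement is enabled, relative to a yaw-only rotation from GetDirection.
; GetDirection uses the far camera's spring arm yaw when the controller uses that camera, otherwise the control rotation.
; The construction script attaches floating log, spotters, warning and stats displays to mesh sockets.
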(event EventBeginPlay
  (|CallParentFunction))

(event Collision|EventActorBeginOverlap
  (params (OtherActor :type Actor%20Object%20Reference)))

(event EventTick
  (params (DeltaSeconds :type Float%20%28single-precision%29)))

(event Input|ActionEvents|InputActionJump
  (params (Key :type Key%20Structure :default "AnyKey"))
  ;[1 1 1] JumpInput
  (:Pressed
    (Character|Jump))
  (:Released
    (Character|StopJumping)))

(event Input|AxisEvents|InputAxisMoveFoward
  (params (AxisValue :type Float%20%28single-precision%29))
  ;[1 1 1] MovementInput
  (if (Variables|Default|GetIsMovementEnabled)
    (bind _rotator (CallFunction|GetDirection))
    (Pawn|Input|AddMovementInput (Math|Vector|GetForwardVector _rotator) AxisValue false)))

(event Input|AxisEvents|InputAxisMoveRight
  (params (AxisValue :type Float%20%28single-precision%29))
  ;[1 1 1] MovementInput
  (if (Variables|Default|GetIsMovementEnabled)
    (bind _rotator (CallFunction|GetDirection))
    (Pawn|Input|AddMovementInput (Math|Vector|GetRightVector _rotator) AxisValue false)))

(fn ConstructionScript
  (|CallParentFunction)
  (Transformation|AttachComponentToComponent (Variables|Default|GetFloatingInfo_Log) (Variables|Character|GetMesh) "LogSocket" "KeepRelative" "KeepRelative" "KeepRelative" true)
  (Transformation|AttachComponentToComponent (Variables|Default|GetFloatingInfo_Spotters) (Variables|Character|GetMesh) "SpottersSocket" "KeepRelative" "KeepRelative" "KeepRelative" true)
  (Transformation|AttachComponentToComponent (Variables|Default|GetFloatingInfo_Warning) (Variables|Character|GetMesh) "WarningSocket" "KeepRelative" "KeepRelative" "KeepRelative" true)
  (Transformation|AttachComponentToComponent (Variables|Default|GetFloatingInfo_Stats) (Variables|Character|GetMesh) "StatsSocket" "KeepRelative" "KeepRelative" "KeepRelative" true))

(fn GetDirection
  (if (Variables|/Game/Characters/BP_PlayerController.BP_PlayerController_C|GetIsUsingFarCamera (Variables|Default|GetControllerRef))
    (return (Math|Rotator|MakeRotator 0.0 0.0 (.yaw (Transformation|GetWorldRotation (Variables|/Game/Characters/FarCam/BP_FarCam_Pawn.BP_FarCam_Pawn_C|GetSpringArm (Variables|/Game/Characters/BP_PlayerController.BP_PlayerController_C|GetFarCamRef (Variables|Default|GetControllerRef)))))))
    (else
      (return (Math|Rotator|MakeRotator 0.0 0.0 (.yaw (Pawn|GetControlRotation :!class /Script/Engine.Pawn)))))))