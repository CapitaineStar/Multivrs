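; Luminous prey creature Blueprint, a child class whose Tick and construction script only call the parent.
; Its SetVisuals event checks IsInSameUniverse but performs no action on the result.
; Disconnected, never-executed logic would swap the mesh to a ghost material or create head and feather dynamic materials, setting their light intensity and blacking out both antler particle effects.
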(event EventTick
  (params (DeltaSeconds :type Float%20%28single-precision%29))
  (|CallParentFunction DeltaSeconds))

(event EventSetVisuals
  (Utilities|FlowControl|Sequence
    (:then_0
      (if (Variables|Default|GetIsInSameUniverse)
        _))))

(fn ConstructionScript
  (|CallParentFunction))