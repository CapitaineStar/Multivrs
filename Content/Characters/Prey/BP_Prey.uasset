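; BP_Prey is the hunted target, which glides along a path from its PathManager by interpolating toward the manager's prey location.
; Its difficulty-sized entropy bubble uses a distance curve to dilate the player's time and raise the game mode's entropy multiplier.
; A projectile hit shows the end-game widget if player and prey share a universe.
; Otherwise, the first hit spawns a fragment and turns the shadow into a ghost, disabling the bubble's effects.
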(event OnComponentBeginOverlap(EntropyBubble)
  (params (OverlappedComponent :type Primitive%20Component%20Object%20Reference) (OtherActor :type Actor%20Object%20Reference) (OtherComp :type Primitive%20Component%20Object%20Reference) (OtherBodyIndex :type Integer) (bFromSweep :type Boolean) (SweepResult :type Hit%20Result%20Structure%20%28by%20ref%29))
  (bind _asbp_player (Utilities|Casting|CastToBP_Player OtherActor))
  (bind _output_get (Variables|References|SetPlayerRef _asbp_player))
  (Default|EnterPreyProximity _output_get)
  (Variables|Default|SetIsHunterInBubble true))

(event OnComponentEndOverlap(EntropyBubble)
  (params (OverlappedComponent :type Primitive%20Component%20Object%20Reference) (OtherActor :type Actor%20Object%20Reference) (OtherComp :type Primitive%20Component%20Object%20Reference) (OtherBodyIndex :type Integer))
  (bind _asbp_player (Utilities|Casting|CastToBP_Player OtherActor))
  (Variables|/Script/Engine.Actor|SetCustomTimeDilation _asbp_player 1.0)
  (Variables|/Game/Foundation/MultivrsGameMode.MultivrsGameMode_C|SetPreyEntropyMultiplier (Variables|References|GetGameModeRef) 1.0)
  (Variables|References|SetPlayerRef (Utilities|Null))
  (Variables|Default|SetIsHunterInBubble false))

(event EventBeginPlay
  (Utilities|FlowControl|Sequence
    (:then_0
      ;[1 1 1] Set references
      (bind _asmultivrs_game_mode (Utilities|Casting|CastToMultivrsGameMode (Game|GetGameMode)))
      (bind _output_get (Variables|References|SetGameModeRef _asmultivrs_game_mode))
      (Variables|References|SetGameInstanceRef (Variables|/Game/Foundation/MultivrsGameMode.MultivrsGameMode_C|GetGameInstanceRef _output_get)))
    (:then_1
      ;[1 1 1] Set Entropy bubble
      (bind _output_get_2 (Variables|Default|SetEntropyRadius (.Prey_EntropyRadius (Utilities|Struct|BreakGameVariables (Default|GetCurrentDifficulty (Variables|References|GetGameInstanceRef))))))
      (Variables|Default|SetEntropyMultiplier (.Prey_EntropyMultiplier (Utilities|Struct|BreakGameVariables (Default|GetCurrentDifficulty (Variables|References|GetGameInstanceRef)))))
      (Components|Sphere|SetSphereRadius (Variables|Default|GetEntropyBubble) _output_get_2 false))
    (:then_2
      ;[1 1 1] Set visuals
      (Variables|Default|SetIsInSameUniverse (== (Variables|/Game/Foundation/MultivrsGameInstance.MultivrsGameInstance_C|GetPlayerUniverse (Variables|References|GetGameInstanceRef)) (Variables|/Game/Foundation/MultivrsGameInstance.MultivrsGameInstance_C|GetPreyUniverse (Variables|References|GetGameInstanceRef))))
      (CallFunction|SetVisuals))))

(event EventTick
  (params (DeltaSeconds :type Float%20%28single-precision%29))
  (if (Variables|Default|GetIsMoving)
    (CallFunction|MoveonPath DeltaSeconds))
  (Variables|References|GetPlayerRef
    (:then
      (CallFunction|ManageEntropyBubble))
    (:else)))

(fn ConstructionScript)

(fn ManageEntropyBubble
  (if (not (Variables|Default|GetIsGhost))
    (Utilities|FlowControl|Sequence
      (:then_0
        ;[1 1 1] Calculate distance ratio
        (LocalVariables|Set_DistanceRatio (/ (Math|Vector|VectorLength (- (Transformation|GetActorLocation) (Transformation|GetActorLocation (Variables|References|GetPlayerRef)))) (Variables|Default|GetEntropyRadius))))
      (:then_1
        ;[1 1 1] Set Time dilation
        (bind _output_get (LocalVariables|Set_CurveValue (Math|Curves|GetFloatValue (Variables|Default|GetEntropyBubbleRamp) (LocalVariables|Get_DistanceRatio))))
        (Variables|/Script/Engine.Actor|SetCustomTimeDilation (Variables|References|GetPlayerRef) _output_get))
      (:then_2
        ;[1 1 1] Set Entropy multiplier
        (Variables|/Game/Foundation/MultivrsGameMode.MultivrsGameMode_C|SetPreyEntropyMultiplier (Variables|References|GetGameModeRef) (+ (* (- 1.0 (LocalVariables|Get_CurveValue)) (Variables|Default|GetEntropyMultiplier)) 1.0))))))

(fn ProjectileHit
  (params (Projectile :type Projectile%20Object%20Reference))
  (bind _returnvalue (Game|GetPlayerCharacter 0))
  (if (and (not (Variables|Default|GetIsInSameUniverse)) (not (Variables|Default|GetIsGhost)))
    ;[1 1 1] Spawn fragment and ghost if Prey shadow is hit
    (Game|SpawnActorfromClass "/Game/Characters/Prey/Prey_Fragment.Prey_Fragment_C" (Math|Conversions|ToTransform(Vector) (Transformation|GetActorLocation)) "Undefined" 0 0)
    (Variables|Default|SetIsGhost true)
    (bind _playerref (Variables|References|GetPlayerRef)
      (:then
        (Variables|/Script/Engine.Actor|SetCustomTimeDilation _playerref 1.0))
      (:else
        _))
    (Variables|/Game/Foundation/MultivrsGameMode.MultivrsGameMode_C|SetPreyEntropyMultiplier (Variables|References|GetGameModeRef) 1.0)
    (CallFunction|SetVisuals)
    (elif (Variables|Default|GetIsInSameUniverse)
      (bind _asplayer_controller (Utilities|Casting|CastToPlayerController (Pawn|GetController _returnvalue)))
      (bind _returnvalue_2 (UserInterface|CreateWidget "/Game/UI/Widget_EndGame.Widget_EndGame_C" _asplayer_controller))
      (bind _asbp_player (Utilities|Casting|CastToBP_Player _returnvalue))
      (Default|DisplayWidget _asbp_player _returnvalue_2 true true))))

(fn InitializePath
  (params (PathManager :type Spline%20Path%20Manager%20Object%20Reference))
  (bind _output_get (Variables|References|SetPathManagerRef PathManager))
  (Variables|/Game/Gameplay/Misc/SplinePathManager.SplinePathManager_C|SetPreyRef _output_get self)
  (Default|CreateNewPath (Variables|References|GetPathManagerRef) (Transformation|GetActorLocation) true)
  (Variables|Default|SetIsMoving true)
  (Default|StartManagePreyPath (Variables|References|GetPathManagerRef)))

(fn MoveonPath
  (params (DeltaTime :type Float%20%28single-precision%29))
  (LocalVariables|Set_DeltaTime DeltaTime)
  (bind _pathmanagerref (Variables|References|GetPathManagerRef)
    (:then
      (Transformation|SetActorLocationAndRotation (Math|Interpolation|VInterpTo (Transformation|GetActorLocation) (Transformation|GetWorldLocation (Variables|/Game/Gameplay/Misc/SplinePathManager.SplinePathManager_C|GetPreyLocation _pathmanagerref)) (LocalVariables|Get_DeltaTime) 1e+01) (Math|Interpolation|RInterpTo (Transformation|GetActorRotation) (Transformation|GetWorldRotation (Variables|/Game/Gameplay/Misc/SplinePathManager.SplinePathManager_C|GetPreyLocation _pathmanagerref)) (LocalVariables|Get_DeltaTime) 0.0)))
    (:else)))

(fn SetVisuals)