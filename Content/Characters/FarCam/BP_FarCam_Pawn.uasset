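; BP_FarCam_Pawn is a distant overview camera pawn that keeps turning to face the player or an override location.
; SetupFarCamera centers it on a sphere bound, then derives spring arm length from radius, FOV and viewport aspect so the sphere fits, with a raised, downward tilt and yaw offset.
; Each Tick, AutoLookAt feeds the override point or the controller's PlayerRef location to LookAtLocation, which eases the spring arm's yaw via RInterpTo.
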(event EventBeginPlay
  (bind _asbp_player_controller (Utilities|Casting|CastToBP_PlayerController (Game|GetPlayerController 0)))
  (Variables|Default|SetControllerRef _asbp_player_controller))

(event EventTick
  (params (DeltaSeconds :type Float%20%28single-precision%29))
  (CallFunction|AutoLookat DeltaSeconds))

(fn ConstructionScript)

(fn SetupFarCamera
  (params (CameraBounds :type Sphere%20Component%20Object%20Reference) (SourceLocation :type Vector) (CameraYawOffset :type Float%20%28single-precision%29))
  (bind _returnvalue (Viewport|GetViewportSize))
  (bind _springarm (Variables|Default|GetSpringArm))
  (LocalVariables|Set_CamYaw CameraYawOffset)
  (Transformation|SetActorLocation (Transformation|GetWorldLocation CameraBounds) false false)
  (CallFunction|LookatLocation SourceLocation 1e+03)
  (bind _output_get (LocalVariables|Set_CamDistance (* (/ (Variables|/Script/Engine.SphereComponent|GetSphereRadius CameraBounds) (Math|Trig|Tan(Degrees) (/ (Variables|/Script/Engine.CameraComponent|GetFieldOfView (Variables|Default|GetCamera)) 2.0))) 1.5 (/ (.x _returnvalue) (.y _returnvalue)))))
  ;[1 1 1] Set spring arm and camera to look slighty from above
  (Variables|/Script/Engine.SpringArmComponent|SetTargetArmLength _springarm _output_get)
  (Variables|/Script/Engine.SpringArmComponent|SetTargetOffset _springarm (Math|Vector|MakeVector 0.0 0.0 (/ _output_get 4.0)))
  (Transformation|SetRelativeRotation (Variables|Default|GetCamera) (Math|Rotator|MakeRotator 0.0 (* (/ (/ _output_get 4.0) (LocalVariables|Get_CamDistance)) -45.0) (LocalVariables|Get_CamYaw)) false false))

(fn LookatLocation
  (params (LookAtLocation :type Vector) (DeltaTime :type Float%20%28single-precision%29))
  (Transformation|SetWorldRotation (Variables|Default|GetSpringArm) (Math|Interpolation|RInterpTo (Transformation|GetWorldRotation (Variables|Default|GetSpringArm)) (Math|Rotator|MakeRotator 0.0 0.0 (.Yaw (Math|Rotator|BreakRotator (Math|Rotator|MakeRotfromX (- (Transformation|GetActorLocation) LookAtLocation))))) DeltaTime (Variables|Default|GetRotateSpeed)) false false))

(fn AutoLookat
  (params (InputPin :type Float%20%28single-precision%29))
  (LocalVariables|Set_DeltaTime InputPin)
  (if (Variables|Default|GetIsLookAtOverride)
    (CallFunction|LookatLocation (Variables|Default|GetLookAtOverrideLocation) (LocalVariables|Get_DeltaTime))
    (else
      (bind _controllerref (Variables|Default|GetControllerRef)
        (:then
          (bind _playerref (Variables|/Game/Characters/BP_PlayerController.BP_PlayerController_C|GetPlayerRef _controllerref)
            (:then
              (CallFunction|LookatLocation (Transformation|GetActorLocation _playerref) (LocalVariables|Get_DeltaTime)))
            (:else)))
        (:else)))))