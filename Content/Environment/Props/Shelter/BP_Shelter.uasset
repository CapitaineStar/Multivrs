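; BP_Shelter is an enterable shelter prop that prompts the player to press E and changes the camera nearby.
; An interaction overlap registers the shelter as the player's overlapped actor and shows floating help text.
; The generic interact event calls EnterShelter on the player and destroys the prompt.
; A second overlap has the player controller switch to a bounded, yaw-offset far camera, then back to the player view on exit.
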(event OnComponentBeginOverlap(Overlap_Interact)
  (params (OverlappedComponent :type Primitive%20Component%20Object%20Reference) (OtherActor :type Actor%20Object%20Reference) (OtherComp :type Primitive%20Component%20Object%20Reference) (OtherBodyIndex :type Integer) (bFromSweep :type Boolean) (SweepResult :type Hit%20Result%20Structure%20%28by%20ref%29))
  ;[1 1 1] Overlap interact
  (bind _asbp_player (Utilities|Casting|CastToBP_Player OtherActor))
  (bind _output_get (Variables|Default|SetPlayerRef _asbp_player))
  (Variables|/Game/Characters/BP_Player.BP_Player_C|SetOverlappedActorRef _output_get self)
  ;[1 1 1] Help text display
  (bind _index (Default|DisplayText (Variables|Default|GetFloatingTextManager) (Utilities|Struct|MakeFloatingTextParameters "NewEnumerator1" (Variables|Default|GetFloatingTextManager) true 1.5e+02 3e+02 1e+02 "(X=-1.000000,Y=-1.000000)") (Utilities|Array|MakeArray (Utilities|String|ToString(Text) (Utilities|Text|MakeLiteralText "Press <E> to enter")))))
  (Variables|Default|SetHelpTextIndex _index))

(event OnComponentEndOverlap(Overlap_Interact)
  (params (OverlappedComponent :type Primitive%20Component%20Object%20Reference) (OtherActor :type Actor%20Object%20Reference) (OtherComp :type Primitive%20Component%20Object%20Reference) (OtherBodyIndex :type Integer))
  ;[1 1 1] Overlap interact
  (bind _asbp_player (Utilities|Casting|CastToBP_Player OtherActor))
  (Variables|/Game/Characters/BP_Player.BP_Player_C|SetOverlappedActorRef _asbp_player 0)
  ;[1 1 1] Help text display
  (Default|FadeOutText (Variables|Default|GetFloatingTextManager) (Variables|Default|GetHelpTextIndex))
  (Variables|Default|SetHelpTextIndex -1))

(event OnComponentBeginOverlap(Overlap_FarCam)
  (params (OverlappedComponent :type Primitive%20Component%20Object%20Reference) (OtherActor :type Actor%20Object%20Reference) (OtherComp :type Primitive%20Component%20Object%20Reference) (OtherBodyIndex :type Integer) (bFromSweep :type Boolean) (SweepResult :type Hit%20Result%20Structure%20%28by%20ref%29))
  ;[1 1 1] Far camera overlap
  (bind _asbp_player (Utilities|Casting|CastToBP_Player OtherActor))
  (Default|SwitchtoFarCam (Variables|Default|GetControllerRef) (Variables|Default|GetOverlap_FarCam) (Transformation|GetActorLocation _asbp_player) 2e+01))

(event OnComponentEndOverlap(Overlap_FarCam)
  (params (OverlappedComponent :type Primitive%20Component%20Object%20Reference) (OtherActor :type Actor%20Object%20Reference) (OtherComp :type Primitive%20Component%20Object%20Reference) (OtherBodyIndex :type Integer))
  ;[1 1 1] Far camera overlap
  (Default|SwitchtoPlayer (Variables|Default|GetControllerRef)))

(event EventBeginPlay
  (bind _asbp_player_controller (Utilities|Casting|CastToBP_PlayerController (Game|GetPlayerController 0)))
  (Variables|Default|SetControllerRef _asbp_player_controller))

(event EventGenericInteractwithSomething
  (Default|EnterShelter (Variables|Default|GetPlayerRef) self)
  ;[1 1 1] Help text display
  (Default|DestroyText (Variables|Default|GetFloatingTextManager) (Variables|Default|GetHelpTextIndex)))

(fn ConstructionScript)