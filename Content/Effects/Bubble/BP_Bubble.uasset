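; BP_Bubble is a bubble visual effect built from a sphere and two counter-rotating attractor meshes.
; Construction creates dynamic material instances for all three and applies shared color and opacity, with slightly offset strand speeds on the attractors.
; Tick spins the attractors in opposite directions at slightly different rates.
; Implode clears the hidden flag and plays a timeline that drives root scale and refreshes material opacity.
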(event Custom|Implode
  (Variables|Default|SetIsHidden false)
  (bind (_direction _scalemultiplier _opacity) (Timeline|Timeline_Implode Play)
    (:Update
      (Transformation|SetRelativeScale3D (Variables|Default|GetDefaultSceneRoot) (Math|Conversions|ToVector(Float) _scalemultiplier))
      (Variables|MaterialParameters|SetOpacity _opacity)
      (CallFunction|SetMatParameters))))

(event EventTick
  (params (DeltaSeconds :type Float%20%28single-precision%29))
  (bind _rotationrate (Variables|MaterialParameters|GetRotationRate))
  (Transformation|AddRelativeRotation (Variables|Default|GetAttractor) (Math|Rotator|MakeRotator 0.0 0.0 (+ _rotationrate (/ _rotationrate 5.0))) false false)
  (Transformation|AddRelativeRotation (Variables|Default|GetAttractor_Flipped) (Math|Rotator|MakeRotator 0.0 0.0 (* (Variables|MaterialParameters|GetRotationRate) -1.0)) false false))

(fn ConstructionScript
  (CallFunction|CreateMatInstances)
  (CallFunction|SetMatParameters))

(fn SetMatParameters
  (bind _strandsspeed (Variables|MaterialParameters|GetStrandsSpeed))
  (Utilities|FlowControl|Sequence
    (:then_0
      ;[1 1 1] Set speed
      (Rendering|Material|SetScalarParameterValue (Variables|Default|GetAttractorMatRef) "TimeScale" (Variables|MaterialParameters|GetStrandsSpeed) :!class /Script/Engine.MaterialInstanceDynamic)
      (Rendering|Material|SetScalarParameterValue (Variables|Default|GetAttractorMatRef_Flipped) "TimeScale" (+ _strandsspeed (/ _strandsspeed 5.0)) :!class /Script/Engine.MaterialInstanceDynamic))
    (:then_1
      ;[1 1 1] Set color
      (Rendering|Material|SetVectorParameterValue (Variables|Default|GetAttractorMatRef) "EmissiveColor" (Variables|MaterialParameters|GetColor) :!class /Script/Engine.MaterialInstanceDynamic))
    (:then_2
      ;[1 1 1] Set opacity
      (Rendering|Material|SetScalarParameterValue (Variables|Default|GetAttractorMatRef) "Opacity" (Variables|MaterialParameters|GetOpacity) :!class /Script/Engine.MaterialInstanceDynamic))))

(fn CreateMatInstances
  (Utilities|FlowControl|Sequence
    (:then_0
      (Utilities|IsValid (Variables|Default|GetAttractorMatRef)
        (:Is%20Not%20Valid
          (bind _returnvalue (Rendering|Material|CreateDynamicMaterialInstance (Variables|Default|GetAttractor) 0 0 :!class /Script/Engine.PrimitiveComponent))
          (Variables|Default|SetAttractorMatRef _returnvalue))))
    (:then_1
      (Utilities|IsValid (Variables|Default|GetAttractorMatRef_Flipped)
        (:Is%20Not%20Valid
          (bind _returnvalue_2 (Rendering|Material|CreateDynamicMaterialInstance (Variables|Default|GetAttractor_Flipped) 0 "/Game/Effects/Bubble/M_AttractorEffect.M_AttractorEffect" :!class /Script/Engine.PrimitiveComponent))
          (Variables|Default|SetAttractorMatRef_Flipped _returnvalue_2))))
    (:then_2
      (Utilities|IsValid (Variables|Default|GetSphereMatRef)
        (:Is%20Not%20Valid
          (bind _returnvalue_3 (Rendering|Material|CreateDynamicMaterialInstance (Variables|Default|GetSphere) 0 "/Game/Effects/Bubble/M_SphereFade.M_SphereFade" :!class /Script/Engine.PrimitiveComponent))
          (Variables|Default|SetSphereMatRef _returnvalue_3))))))