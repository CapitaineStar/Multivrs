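; Spotter effect decal that indicates the direction of the prey's momentum, read from the MultivrsGameMode.
; A dynamic material instance drives the decal, with a timeline animating its Radius on spawn and Tick turning the actor to follow PreyMomentum.
; SetOffset and DisableOffset temporarily shift and scale the actor, then restore or relocate it at unit scale.
; SelfDestruct schedules a decal fade-out that destroys the actor when done.
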(event Custom|SelfDestruct
  (params (Delay :type Float%20%28single-precision%29))
  (bind _fadeoutduration (Variables|Default|GetFadeOutDuration))
  (Rendering|Components|Decal|SetFadeOut (Variables|Decal|GetDecal) (- Delay _fadeoutduration) _fadeoutduration true))

(event EventBeginPlay
  (bind _asmultivrs_game_mode (Utilities|Casting|CastToMultivrsGameMode (Game|GetGameMode)))
  (Variables|Default|SetGameModeRef _asmultivrs_game_mode)
  (bind _radius (Timeline|MaterialFade Play)
    (:Update
      (Rendering|Material|SetScalarParameterValue (Variables|Default|GetMaterialRef) "Radius" _radius :!class /Script/Engine.MaterialInstanceDynamic))))

(event EventTick
  (params (DeltaSeconds :type Float%20%28single-precision%29))
  (bind _gamemoderef (Variables|Default|GetGameModeRef)
    (:then
      (Transformation|SetActorRotation (Math|Rotator|MakeRotator 0.0 9e+01 (+ (Variables|/Game/Foundation/MultivrsGameMode.MultivrsGameMode_C|GetPreyMomentum _gamemoderef) 9e+01))))
    (:else)))

(fn ConstructionScript
  (Rendering|Components|Decal|SetDecalMaterial (Variables|Decal|GetDecal) "/Game/Effects/Spotters/M_Effect_Momentum.M_Effect_Momentum")
  (bind _returnvalue (Rendering|Material|CreateDynamicMaterialInstance (Variables|Decal|GetDecal) :!class /Script/Engine.DecalComponent))
  (Variables|Default|SetMaterialRef _returnvalue))

(fn SetOffset
  (params (Offset :type Vector) (UniformScale :type Float%20%28single-precision%29))
  (bind _output_get (Variables|Default|SetOffset Offset))
  (Transformation|SetActorLocation (+ _output_get (Transformation|GetActorLocation)) false false)
  (Transformation|SetActorScale3D (Math|Vector|MakeVector UniformScale UniformScale UniformScale)))

(fn DisableOffset
  (params (NewLocation :type Vector))
  (if (> (Math|Vector|VectorLength NewLocation) 0.1)
    (Transformation|SetActorLocation NewLocation false false)
    (else
      (Transformation|SetActorLocation (- (Transformation|GetActorLocation) (Variables|Default|GetOffset)) false false)))
  (Transformation|SetActorScale3D "1.0,1.000000,1.000000")
  (Variables|Default|SetOffset "0, 0, 0"))