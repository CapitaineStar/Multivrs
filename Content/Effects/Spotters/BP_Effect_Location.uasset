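; Location effect actor that shows a post-process visual driven by the player's position and the prey's location.
; SetLocationEffect creates a dynamic material, seeds both positions and applies it through the given ambience manager, while Tick keeps the player position current.
; One timeline animates Radius forward to fade in and LinearFade in reverse to fade out.
; SelfDestruct schedules that reversal, which removes the post-process and destroys the actor.
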(event Custom|SelfDestruct
  (params (Delay :type Float%20%28single-precision%29))
  (Utilities|FlowControl|Delay (- Delay (Variables|Default|GetFadeOutDuration)))
  (bind (_direction _radius _linearfade) (Timeline|MaterialFade Reverse)
    (:Update
      (switch Utilities|FlowControl|Switch|SwitchonETimelineDirection _direction
        (:Forward
          (Rendering|Material|SetScalarParameterValue (Variables|References|GetMaterialRef) "Radius" _radius :!class /Script/Engine.MaterialInstanceDynamic))
        (:Backward
          (Rendering|Material|SetScalarParameterValue (Variables|References|GetMaterialRef) "LinearFade" _linearfade :!class /Script/Engine.MaterialInstanceDynamic))))
    (:Finished
      (switch Utilities|FlowControl|Switch|SwitchonETimelineDirection _direction
        (:Backward
          (Default|ApplyPostProcess (Variables|References|GetAmbienceManagerRef) (Variables|References|GetMaterialRef) 0.0)
          (Actor|DestroyActor))))))

(event Custom|FadeIn
  (bind (_direction _radius _linearfade) (Timeline|MaterialFade Play)
    (:Update
      (switch Utilities|FlowControl|Switch|SwitchonETimelineDirection _direction
        (:Forward
          (Rendering|Material|SetScalarParameterValue (Variables|References|GetMaterialRef) "Radius" _radius :!class /Script/Engine.MaterialInstanceDynamic))
        (:Backward
          (Rendering|Material|SetScalarParameterValue (Variables|References|GetMaterialRef) "LinearFade" _linearfade :!class /Script/Engine.MaterialInstanceDynamic))))
    (:Finished
      (switch Utilities|FlowControl|Switch|SwitchonETimelineDirection _direction
        (:Backward
          (Default|ApplyPostProcess (Variables|References|GetAmbienceManagerRef) (Variables|References|GetMaterialRef) 0.0)
          (Actor|DestroyActor))))))

(event EventBeginPlay
  (bind _asmultivrs_game_mode (Utilities|Casting|CastToMultivrsGameMode (Game|GetGameMode)))
  (Variables|References|SetGameModeRef _asmultivrs_game_mode))

(event EventTick
  (params (DeltaSeconds :type Float%20%28single-precision%29))
  (bind _materialref (Variables|References|GetMaterialRef)
    (:then
      (Rendering|Material|SetVectorParameterValue _materialref "PlayerWS" (Math|Conversions|ToLinearColor(Vector) (Transformation|GetActorLocation (Variables|/Game/Foundation/MultivrsGameMode.MultivrsGameMode_C|GetPlayerRef (Variables|References|GetGameModeRef)))) :!class /Script/Engine.MaterialInstanceDynamic))
    (:else)))

(fn ConstructionScript)

(fn SetLocationEffect
  (params (AmbienceManager :type Ambience%20Manager%20Object%20Reference))
  (Variables|References|SetAmbienceManagerRef AmbienceManager)
  (Utilities|FlowControl|Sequence
    (:then_0
      (bind _returnvalue (Rendering|Material|CreateDynamicMaterialInstance "/Game/Effects/Spotters/M_Effect_Location.M_Effect_Location" :!class /Script/Engine.KismetMaterialLibrary))
      (Variables|References|SetMaterialRef _returnvalue)
      (Rendering|Material|SetVectorParameterValue (Variables|References|GetMaterialRef) "PlayerWS" (Math|Conversions|ToLinearColor(Vector) (Transformation|GetActorLocation (Variables|/Game/Foundation/MultivrsGameMode.MultivrsGameMode_C|GetPlayerRef (Variables|References|GetGameModeRef)))) :!class /Script/Engine.MaterialInstanceDynamic)
      (Rendering|Material|SetVectorParameterValue (Variables|References|GetMaterialRef) "LocationWS" (Math|Conversions|ToLinearColor(Vector) (Default|GetPreyLocation (Variables|References|GetGameModeRef))) :!class /Script/Engine.MaterialInstanceDynamic)
      (Rendering|Material|SetScalarParameterValue (Variables|References|GetMaterialRef) "Radius" 1.0 :!class /Script/Engine.MaterialInstanceDynamic))
    (:then_1
      (Default|ApplyPostProcess (Variables|References|GetAmbienceManagerRef) (Variables|References|GetMaterialRef) 1.0)
      (CallFunction|Fadein))))