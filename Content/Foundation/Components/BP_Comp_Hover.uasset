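; BP_Comp_Hover is a component that gives its owning actor a hovering wobble.
; On BeginPlay it caches a PrimitiveComponent from the owner, then sets that component's relative location every Tick.
; Each axis follows a degree-based sine of a wrapping timer, scaled by Amplitude, with slightly offset Speed values so the axes drift out of phase.
; The motion centers on the relative origin, replacing any initial offset.
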(event EventBeginPlay
  (Variables|Default|SetPrimitiveRef (Actor|GetComponentbyClass (Components|GetOwner) "/Script/Engine.PrimitiveComponent")))

(event EventTick
  (params (DeltaSeconds :type Float%20%28single-precision%29))
  (bind _speed (Variables|Hover|GetSpeed))
  (bind _amplitude (Variables|Hover|GetAmplitude))
  (bind _output_get (Variables|Default|SetTimer (Math|Float|%(Float) (+ DeltaSeconds (Variables|Default|GetTimer)) 3.6e+02)))
  (Transformation|SetRelativeLocation (Variables|Default|GetPrimitiveRef) (Math|Vector|MakeVector (* (Math|Trig|Sin(Degrees) (* _output_get (+ _speed 0.15))) _amplitude) (* _amplitude (Math|Trig|Sin(Degrees) (* _output_get _speed))) (* _amplitude (Math|Trig|Sin(Degrees) (* _output_get (+ _speed -0.2))))) false false))