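; Actor component that manages on-screen floating text widgets, offering calls to show, update, fade out or destroy them.
; DisplayText creates a Widget_FloatingText, applies its parameters and text, adds it to the viewport and returns its array index as the handle.
; Fade and destroy calls also remove the array entry, so handles to later texts shift and can go stale.
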(event EventBeginPlay)

(event EventTick
  (params (DeltaSeconds :type Float%20%28single-precision%29)))

(fn DisplayText
  (params (Parameters :type Floating%20Text%20Parameters%20Structure) (MultilineText :type Array%20of%20Strings))
  (bind _returnvalue (UserInterface|CreateWidget "/Game/UI/Widget_FloatingText.Widget_FloatingText_C"))
  (bind _returnvalue_2 (Utilities|Array|Add (Variables|Default|GetFloatingTexts) _returnvalue))
  (Default|SetParameters _returnvalue Parameters MultilineText)
  (UserInterface|Viewport|AddtoViewport _returnvalue 0)
  (return _returnvalue_2))

(fn FadeOutText
  (params (Index :type Integer))
  (bind _output_get (LocalVariables|Set_Index Index))
  (if (Utilities|Array|IsValidIndex (Variables|Default|GetFloatingTexts) _output_get)
    (Default|FadeOut (Utilities|Array|Get(acopy) (Variables|Default|GetFloatingTexts) (LocalVariables|Get_Index)))
    (Utilities|Array|RemoveIndex (Variables|Default|GetFloatingTexts) (LocalVariables|Get_Index))))

(fn DestroyText
  (params (Index :type Integer))
  (bind _output_get (LocalVariables|Set_Index Index))
  (if (Utilities|Array|IsValidIndex (Variables|Default|GetFloatingTexts) _output_get)
    (Default|Destroy (Utilities|Array|Get(acopy) (Variables|Default|GetFloatingTexts) (LocalVariables|Get_Index)))
    (Utilities|Array|RemoveIndex (Variables|Default|GetFloatingTexts) (LocalVariables|Get_Index))))

(fn FadeOutTexts
  (params (Indexes :type Array%20of%20Integers))
  (bind _floatingtexts (Variables|Default|GetFloatingTexts))
  (for _array_element Indexes
    (if (Utilities|Array|IsValidIndex _floatingtexts _array_element)
      (Default|FadeOut (Utilities|Array|Get(acopy) _floatingtexts _array_element))))
  (for _array_element_2 Indexes
    (Utilities|Array|RemoveIndex (Variables|Default|GetFloatingTexts) _array_element_2)))

(fn UpdateText
  (params (Index :type Integer) (MultilineText :type Array%20of%20Strings))
  (if (!= Index -1)
    (Default|SetMultilineText (Utilities|Array|Get(acopy) (Variables|Default|GetFloatingTexts) Index) MultilineText)))