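; Hex tile actor that forms one piece of the world, with biome-driven scale and wind plus spawned spotter items and traps.
; Construction scatters structures across three instanced mesh components, reading transforms from a point mesh's vertex positions and colors.
; SetupHexTile applies game-instance biome, difficulty and hex modifiers, then attaches spawns at random sphere-traced locations.
; Tick hides wind beyond two tiles from the current coordinate, and SelfDestruct removes attached actors with the tile.
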(event Custom|SelfDestruct
  (bind _self self)
  (bind _outactors (Actor|GetAttachedActors _self))
  ;[1 1 1] Self-Destruct
  (Actor|DestroyActor _outactors :!label _label)
  (if (== (Utilities|Array|Length _outactors) 0)
    (Actor|DestroyActor)
    (else
      (goto _label))))

(event EventTick
  (params (DeltaSeconds :type Float%20%28single-precision%29))
  ;[1 1 1] Hide wind effect if too far
  (bind _gamemoderef (Variables|References|GetGameModeRef)
    (:then
      (bind _distance (CallFunction|Distance (Variables|/Game/Foundation/MultivrsGameMode.MultivrsGameMode_C|GetCurrentCoord _gamemoderef)))
      (Rendering|SetVisibility (Variables|Default|GetWind) (<= _distance 2) false))
    (:else)))

(event EventBeginPlay
  ;[1 1 1] Begin play
  (bind _asmultivrs_game_mode (Utilities|Casting|CastToMultivrsGameMode (Game|GetGameMode)))
  (Variables|References|SetGameModeRef _asmultivrs_game_mode)
  (bind _asmultivrs_game_instance (Utilities|Casting|CastToMultivrsGameInstance (Game|GetGameInstance)))
  (Variables|References|SetGameInstanceRef _asmultivrs_game_instance))

(fn ConstructionScript
  (|CallParentFunction)
  (Utilities|FlowControl|Sequence
    (:then_0
      (Components|StaticMesh|SetStaticMesh (Variables|Default|GetGround) (Variables|Variables|GetSM_Ground))
      (Components|StaticMesh|SetStaticMesh (Variables|Default|GetGroundBorder) (Variables|Variables|GetSM_GroundBorder)))
    (:then_1
      (bind _sm_scattererpts (Variables|Variables|GetSM_ScattererPts)
        (:then
          (Components|StaticMesh|SetStaticMesh (Variables|Default|GetScatterPoints) _sm_scattererpts)
          (CallFunction|ScatterStructs))
        (:else)))
    (:then_2
      (bind _sm_wind (Variables|Variables|GetSM_Wind)
        (:then
          (Components|StaticMesh|SetStaticMesh (Variables|Default|GetWind) _sm_wind))
        (:else)))))

(fn SetBiome
  (Utilities|FlowControl|Sequence
    (:then_0
      ;[1 1 1] Set scale
      (Transformation|SetRelativeScale3D (Variables|Default|GetDefaultSceneRoot) (Math|Conversions|ToVector(Float) (.HexTileScale (Utilities|Struct|BreakBiomeDescription (Variables|Default|GetLocalBiome))))))
    (:then_1
      ;[1 1 1] Set wind
      (bind _returnvalue (Rendering|Material|CreateDynamicMaterialInstance (Variables|Default|GetWind) 0 "/Game/Effects/Wind/M_Effect_WindPanner.M_Effect_WindPanner" :!class /Script/Engine.PrimitiveComponent))
      (bind _output_get (Variables|References|SetWindMaterialRef _returnvalue))
      (Rendering|Material|SetScalarParameterValue _output_get "WindSpeed" (* (.WindSpeed (Utilities|Struct|BreakBiomeDescription (Variables|Default|GetLocalBiome))) 0.1) :!class /Script/Engine.MaterialInstanceDynamic)
      (Rendering|Material|SetVectorParameterValue _output_get "Color" (Variables|Default|GetWindColor) :!class /Script/Engine.MaterialInstanceDynamic))))

(fn ScatterStructs
  (bind _instancedsmcomponents (LocalVariables|GetInstancedSMComponents))
  (bind _scatterpoints (Variables|Default|GetScatterPoints))
  (bind _instancedsmcomponents_2 (LocalVariables|GetInstancedSMComponents))
  (bind (_vertexpositions _vertexcolors _returnvalue) (Class|MultivrsBPLibrary|GetStaticMeshVertexInfo _scatterpoints))
  (Utilities|Array|Add _instancedsmcomponents (Variables|Default|GetInstancedSM_Structs0))
  (Utilities|Array|Add _instancedsmcomponents (Variables|Default|GetInstancedSM_Structs1))
  (Utilities|Array|Add _instancedsmcomponents (Variables|Default|GetInstancedSM_Structs2))
  (Utilities|FlowControl|Sequence
    (:then_0
      ;[1 1 1] Create one Instanced SM for every structs
      (for _index (range 0 (- (Utilities|Array|Length (Variables|Variables|GetSM_ScattererStructs)) 1))
        (Components|StaticMesh|SetStaticMesh (Utilities|Array|Get(acopy) (LocalVariables|GetInstancedSMComponents) (Math|Integer|%(Integer) _index 3)) (Utilities|Array|Get(acopy) (Variables|Variables|GetSM_ScattererStructs) _index))))
    (:then_1
      ;[1 1 1] For each scatter points
      (if _returnvalue
        (for (_array_element _array_index) _vertexpositions
          (Utilities|FlowControl|Sequence
            (:then_0
              ;[1 1 1] Make transform from Vertex Color
              (LocalVariables|SetTransform (Math|Transform|MakeTransform _array_element (Math|Rotator|MakeRotator (Math|Trig|RadiansToDegrees (.X (Math|Vector|BreakVector (* (.RGBVector (Utilities|RGBAtoVector4 (Utilities|Array|Get(acopy) _vertexcolors _array_index))) (* (Math|Trig|GetPI) 2.0))))) (Math|Trig|RadiansToDegrees (.Y (Math|Vector|BreakVector (* (.RGBVector (Utilities|RGBAtoVector4 (Utilities|Array|Get(acopy) _vertexcolors _array_index))) (* (Math|Trig|GetPI) 2.0))))) (* (Math|Trig|RadiansToDegrees (.Z (Math|Vector|BreakVector (* (.RGBVector (Utilities|RGBAtoVector4 (Utilities|Array|Get(acopy) _vertexcolors _array_index))) (* (Math|Trig|GetPI) 2.0))))) -1.0)) (Math|Conversions|ToVector(Float) (.Alpha (Utilities|RGBAtoVector4 (Utilities|Array|Get(acopy) _vertexcolors _array_index)))))))
            (:then_1
              ;[1 1 1] Add instance on alternating component
              (Components|InstancedStaticMesh|AddInstance (Utilities|Array|Get(acopy) _instancedsmcomponents_2 (Math|Integer|%(Integer) _array_index (Utilities|Array|Length _instancedsmcomponents_2))) (LocalVariables|GetTransform)))))))))

(fn SpawnSpotters
  (LocalVariables|Set_RandomStart (Math|Conversions|ToInteger(Boolean) (Math|Random|RandomBool)))
  (for _index (range 0 (- (Variables|Default|GetSpottersNum) 1))
    (LocalVariables|Set_i _index)
    (bind (_success _worldlocation) (CallFunction|GetValidLocationonTile))
    (if _success
      (LocalVariables|Set_SpawnLocation _worldlocation)
      ;[1 1 1] Spawn random (alternate) item
      (if (Math|Conversions|ToBoolean(Integer) (Math|Integer|%(Integer) (+ (LocalVariables|Get_i) (LocalVariables|Get_RandomStart)) 2))
        (bind _returnvalue (Game|SpawnActorfromClass "/Game/Gameplay/Pickup/Item/Item_LocationSpotter_00.Item_LocationSpotter_00_C" (Math|Conversions|ToTransform(Vector) (LocalVariables|Get_SpawnLocation)) "Undefined" 0 0))
        (Transformation|AttachActorToActor _returnvalue self "" "KeepWorld" "KeepWorld" "KeepWorld" true)
        (else
          (bind _returnvalue_2 (Game|SpawnActorfromClass "/Game/Gameplay/Pickup/Item/Item_MomentumSpotter_00.Item_MomentumSpotter_00_C" (Math|Conversions|ToTransform(Vector) (LocalVariables|Get_SpawnLocation)) "Undefined" 0 0))
          (Transformation|AttachActorToActor _returnvalue_2 self "" "KeepWorld" "KeepWorld" "KeepWorld" true))))))

(fn SetupHexTile
  (params (Coordinates :type Hex%20Cube%20Coordinates%20Structure) (ObservedHexIndex :type Integer))
  (bind _gameinstanceref (Variables|References|GetGameInstanceRef))
  (bind _currentgamevariables (Default|GetCurrentDifficulty _gameinstanceref))
  (bind (_hex_mindistanceany _hex_mindistanceshelter _hex_mindistanceportal _hex_mindistanceequipment _spotter_nbpertile _trap_nbpertile) (Utilities|Struct|BreakGameVariables _currentgamevariables))
  (Variables|Default|SetCoordinates Coordinates)
  (Variables|Default|SetObservedHexIndex ObservedHexIndex)
  (Variables|References|GetGameInstanceRef
    (:then
      (Utilities|FlowControl|Sequence
        (:then_0
          ;[1 1 1] Set variables
          (Variables|Default|SetLocalBiome (Utilities|MakeLocalBiome))
          (Variables|Default|SetSpottersNum (Math|Float|Round (* _spotter_nbpertile (.SpottersAmount (Utilities|Struct|BreakHexModifier (Default|GetHexModifier (Variables|References|GetGameInstanceRef) (Variables|Default|GetObservedHexIndex)))))))
          (Variables|Default|SetTrapsNum _trap_nbpertile)
          (Variables|Default|SetWindColor (.WindColor (Utilities|Struct|BreakAmbienceDescription (Default|GetCurrentAmbience (Variables|References|GetGameInstanceRef))))))
        (:then_1
          ;[1 1 1] Setup extras
          (CallFunction|SetBiome)
          (CallFunction|SpawnSpotters)
          (CallFunction|SpawnTraps))))
    (:else)))

(fn RefreshHexTile
  (Utilities|FlowControl|Sequence
    (:then_0
      (Variables|Default|SetLocalBiome (Utilities|MakeLocalBiome)))
    (:then_1
      (bind _windmaterialref (Variables|References|GetWindMaterialRef)
        (:then
          (Rendering|Material|SetScalarParameterValue _windmaterialref "WindSpeed" (* (.WindSpeed (Utilities|Struct|BreakBiomeDescription (Variables|Default|GetLocalBiome))) 0.1) :!class /Script/Engine.MaterialInstanceDynamic))
        (:else)))))

(fn GetValidLocationonTile
  (bind _returnvalue (Transformation|GetActorLocation))
  (bind _returnvalue_2 (Math|Vector|MakeVector 0.0 0.0 2e+03))
  (bind (_radius _angle__rad_) (Utilities|RandomPolarCoord))
  (bind (_radius_2 _angle__rad__2) (Utilities|RandomPolarCoord))
  (bind _returnvalue_3 (Math|Trig|Sin(Radians) _angle__rad_))
  (bind _returnvalue_4 (Math|Trig|Cos(Radians) _angle__rad__2))
  (bind _returnvalue_5 (* _radius _returnvalue_3))
  (bind _returnvalue_6 (* _radius_2 _returnvalue_4))
  (bind _returnvalue_7 (Math|Vector|MakeVector _returnvalue_6 _returnvalue_5 0.0))
  (bind _returnvalue_8 (+ _returnvalue_7 _returnvalue))
  ;[1 1 1] Prevent infinite attempts
  (for _index (range 0 (Class|KismetSystemLibrary|MakeLiteralInteger 5))
    (Utilities|FlowControl|Sequence
      (:then_0
        ;[1 1 1] Get potential location on tile surface
        (bind (_outhit _returnvalue_9) (Collision|SphereTraceForObjects (+ _returnvalue_8 _returnvalue_2) (- _returnvalue_8 _returnvalue_2) 1.2e+02 (Utilities|Array|MakeArray "ObjectTypeQuery1") false 0 "None" false))
        (if _returnvalue_9
          (LocalVariables|Set_PotentialLocation (.Location (Collision|BreakHitResult _outhit)))))
      (:then_1
        ;[1 1 1] Check if near non-valid dynamic object
        (bind (_outhit_2 _returnvalue_10) (Collision|SphereTraceForObjects (LocalVariables|Get_PotentialLocation) (- (LocalVariables|Get_PotentialLocation) "0, 0,100.000000") 1e+03 (Utilities|Array|MakeArray "ObjectTypeQuery2" "ObjectTypeQuery3") false 0 "None"))
        (if _returnvalue_10
          (if (not (Math|Boolean|ORBoolean (.bSuccess (Utilities|Casting|CastToBP_Pickup (.HitActor (Collision|BreakHitResult _outhit_2)))) (.bSuccess (Utilities|Casting|CastToBP_Trap (.HitActor (Collision|BreakHitResult _outhit_2)))) (.bSuccess (Utilities|Casting|CastToBP_Portal (.HitActor (Collision|BreakHitResult _outhit_2)))) (.bSuccess (Utilities|Casting|CastToBP_Shelter (.HitActor (Collision|BreakHitResult _outhit_2))))))
            (return true (LocalVariables|Get_PotentialLocation)))
          (else
            (return true (LocalVariables|Get_PotentialLocation)))))))
  (return false "0, 0, 0"))

(fn SpawnTraps
  (for _index (range 0 (- (Variables|Default|GetTrapsNum) 1))
    (LocalVariables|Set_i _index)
    (bind (_success _worldlocation) (CallFunction|GetValidLocationonTile))
    (if _success
      (LocalVariables|Set_SpawnLocation _worldlocation)
      ;[1 1 1] Spawn trap
      (bind _returnvalue (Game|SpawnActorfromClass "/Game/Gameplay/Trap/BP_Trap.BP_Trap_C" (Math|Conversions|ToTransform(Vector) (LocalVariables|Get_SpawnLocation)) "Undefined" 0 0))
      (Transformation|AttachActorToActor _returnvalue self "" "KeepWorld" "KeepWorld" "KeepWorld" true))))