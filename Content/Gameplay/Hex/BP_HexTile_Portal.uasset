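; Hex tile variant that places a portal on the board.
; When its hex type is set up, it spawns a BP_Portal at the PortalLocation component's world location and rotation, with unit scale.
; The portal is stored, attached to the tile with world transforms kept, then initialized with the tile's Coordinates.
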(event EventSetupHexType
  (CallFunction|SpawnPortal))

(fn ConstructionScript
  (|CallParentFunction))

(fn SpawnPortal
  (bind _portallocation (Variables|Default|GetPortalLocation))
  (Utilities|FlowControl|Sequence
    (:then_0
      ;[1 1 1] Spawn portal
      (bind _returnvalue (Game|SpawnActorfromClass "/Game/Environment/Props/Portal/BP_Portal.BP_Portal_C" (Math|Transform|MakeTransform (Transformation|GetWorldLocation _portallocation) (Transformation|GetWorldRotation _portallocation)) "Undefined" 0 0))
      (bind _output_get (Variables|Default|SetPortalRef _returnvalue))
      (Transformation|AttachActorToActor _output_get self "EquipmentLocation" "KeepWorld" "KeepWorld" "KeepWorld" true))
    (:then_1
      (Default|SetupPortal (Variables|Default|GetPortalRef) (Variables|Default|GetCoordinates)))))