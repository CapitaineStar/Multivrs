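; BP_Hex is a hex grid cell Blueprint that holds cube coordinates and provides the math for working with them.
; Add, Substract and Scale return new coordinates, and Equals compares a given coordinate with its own.
; Direction maps six compass headings to unit offsets, which Neighbor adds to find the adjacent coordinate.
; Distance halves the summed absolute components of the difference from Substract to give hex steps.
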(fn ConstructionScript)

(fn Add
  (params (HexIn :type Hex%20Cube%20Coordinates%20Structure))
  (bind (_x _y _z) (Utilities|Struct|BreakHexCubeCoordinates HexIn))
  (bind _coordinates (Variables|Variables|GetCoordinates))
  (bind (_x_2 _y_2 _z_2) (Utilities|Struct|BreakHexCubeCoordinates _coordinates))
  (return (Utilities|Struct|MakeHexCubeCoordinates (+ _x _x_2) (+ _y _y_2) (+ _z _z_2))))

(fn Substract
  (params (HexIn :type Hex%20Cube%20Coordinates%20Structure))
  (bind (_x _y _z) (Utilities|Struct|BreakHexCubeCoordinates HexIn))
  (bind _coordinates (Variables|Variables|GetCoordinates))
  (bind (_x_2 _y_2 _z_2) (Utilities|Struct|BreakHexCubeCoordinates _coordinates))
  (return (Utilities|Struct|MakeHexCubeCoordinates (- _x _x_2) (- _y _y_2) (- _z _z_2))))

(fn Scale
  (params (ScaleFactor :type Integer))
  (bind _coordinates (Variables|Variables|GetCoordinates))
  (bind (_x _y _z) (Utilities|Struct|BreakHexCubeCoordinates _coordinates))
  (return (Utilities|Struct|MakeHexCubeCoordinates (* _x ScaleFactor) (* _y ScaleFactor) (* _z ScaleFactor))))

(fn Direction
  (params (Direction :type HexDirection%20Enum))
  (switch Utilities|FlowControl|Switch|SwitchonHexDirection Direction
    (:NewEnumerator0
      (return (Utilities|Struct|MakeHexCubeCoordinates 1 0 -1)))
    (:NewEnumerator1
      (return (Utilities|Struct|MakeHexCubeCoordinates 1 -1)))
    (:NewEnumerator2
      (return (Utilities|Struct|MakeHexCubeCoordinates 0 -1 1)))
    (:NewEnumerator3
      (return (Utilities|Struct|MakeHexCubeCoordinates -1 0 1)))
    (:NewEnumerator4
      (return (Utilities|Struct|MakeHexCubeCoordinates -1 1)))
    (:NewEnumerator5
      (return (Utilities|Struct|MakeHexCubeCoordinates 0 1 -1)))))

(fn Neighbor
  (params (Direction :type HexDirection%20Enum))
  (bind _hexdirection (CallFunction|Direction Direction))
  (bind _hexout (CallFunction|Add _hexdirection))
  (return _hexout))

(fn Distance
  (params (HexIn :type Hex%20Cube%20Coordinates%20Structure))
  (bind _hexout (CallFunction|Substract HexIn))
  (return (/ (+ (Math|Integer|Absolute(Integer) (.x (Utilities|Struct|BreakHexCubeCoordinates _hexout))) (+ (Math|Integer|Absolute(Integer) (.y (Utilities|Struct|BreakHexCubeCoordinates _hexout))) (Math|Integer|Absolute(Integer) (.z (Utilities|Struct|BreakHexCubeCoordinates _hexout))))) 2)))

(fn Equals
  (params (HexIn :type Hex%20Cube%20Coordinates%20Structure))
  (return (CallFunction|Equal(HexCoord) HexIn (Variables|Variables|GetCoordinates))))