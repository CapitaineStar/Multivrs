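; Shelter variant of a hex tile that places a shelter actor on itself when its hex type is set up.
; SetupHexType asks MultivrsGameMode to spawn the shelter rather than spawning it directly.
; A valid shelter is attached to the tile at the EquipmentLocation socket, then teleported to the ShelterLocation component's world position and rotation at unit scale.
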(event EventSetupHexType
  (bind _shelterlocation (Variables|Default|GetShelterLocation))
  ;[1 1 1] Ask to spawn shelter
  (bind _asmultivrs_game_mode (Utilities|Casting|CastToMultivrsGameMode (Game|GetGameMode)))
  (bind _shelterref (Default|SpawnShelter _asmultivrs_game_mode))
  (Utilities|IsValid _shelterref
    (:Is%20Valid
      ;[1 1 1] Set at correct location
      (Transformation|AttachActorToActor _shelterref self "EquipmentLocation" "KeepRelative" "KeepRelative" "KeepRelative" true)
      (Transformation|SetActorTransform _shelterref (Math|Transform|MakeTransform (Transformation|GetWorldLocation _shelterlocation) (Transformation|GetWorldRotation _shelterlocation)) false true))))

(fn ConstructionScript
  (|CallParentFunction))