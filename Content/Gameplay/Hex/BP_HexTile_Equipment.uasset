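; BP_HexTile_Equipment is a hex tile Blueprint that hosts a piece of equipment on the tile.
; Its SetupHexEquipment event asks MultivrsGameMode to spawn the equipment for ObservedHexIndex, so the game mode decides what appears.
; A valid result is attached to the tile and teleported to the world position of the EquipmentLocation component.
; The construction script only calls its parent.
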(event EventSetupHexEquipment
  ;[1 1 1] Ask to spawn correct equipment
  (bind _asmultivrs_game_mode (Utilities|Casting|CastToMultivrsGameMode (Game|GetGameMode)))
  (bind _equipmentref (Default|SpawnEquipment _asmultivrs_game_mode (Variables|Default|GetObservedHexIndex)))
  (Utilities|IsValid _equipmentref
    (:Is%20Valid
      ;[1 1 1] Set at correct location
      (Transformation|AttachActorToActor _equipmentref self "EquipmentLocation" "KeepRelative" "KeepRelative" "KeepRelative" true)
      (Transformation|SetActorTransform _equipmentref (Math|Conversions|ToTransform(Vector) (Transformation|GetWorldLocation (Variables|Default|GetEquipmentLocation))) false true))))

(fn ConstructionScript
  (|CallParentFunction))