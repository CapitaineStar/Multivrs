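; BP_Pickup is a pickup actor that shows a floating text tooltip while the player is nearby.
; Entering the TooltipOverlap sphere displays TooltipText through FloatingTextManager and stores its index, which is used to fade the text on exit or remove it when destroyed.
; The construction script sizes separate pickup and tooltip spheres from radius variables.
; PickupOverlap has no collection logic in this graph.
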(event OnComponentBeginOverlap(TooltipOverlap)
  (params (OverlappedComponent :type Primitive%20Component%20Object%20Reference) (OtherActor :type Actor%20Object%20Reference) (OtherComp :type Primitive%20Component%20Object%20Reference) (OtherBodyIndex :type Integer) (bFromSweep :type Boolean) (SweepResult :type Hit%20Result%20Structure%20%28by%20ref%29))
  (Utilities|Casting|CastToBP_Player OtherActor)
  (bind _index (Default|DisplayText (Variables|Default|GetFloatingTextManager) (Utilities|Struct|MakeFloatingTextParameters "NewEnumerator0" (Variables|Default|GetDefaultSceneRoot)) (Utilities|Array|MakeArray (Utilities|String|ToString(Text) (Variables|Default|GetTooltipText)))))
  (Variables|Default|SetTooltipIndex _index))

(event OnComponentEndOverlap(TooltipOverlap)
  (params (OverlappedComponent :type Primitive%20Component%20Object%20Reference) (OtherActor :type Actor%20Object%20Reference) (OtherComp :type Primitive%20Component%20Object%20Reference) (OtherBodyIndex :type Integer))
  (Utilities|Casting|CastToBP_Player OtherActor)
  (Default|FadeOutText (Variables|Default|GetFloatingTextManager) (Variables|Default|GetTooltipIndex))
  (Variables|Default|SetTooltipIndex -1))

(event EventDestroyed
  (Default|DestroyText (Variables|Default|GetFloatingTextManager) (Variables|Default|GetTooltipIndex))
  (Variables|Default|SetTooltipIndex -1))

(fn ConstructionScript
  (Components|Sphere|SetSphereRadius (Variables|Default|GetPickupOverlap) (Variables|Default|GetPickupRadius) false)
  (Components|Sphere|SetSphereRadius (Variables|Default|GetTooltipOverlap) (Variables|Default|GetTooltipRadius) false))