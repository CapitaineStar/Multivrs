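; Base equipment pickup that the player takes by interacting, with data read from the GameInstance's ObservedEquipments by index.
; Overlap registers it with BP_Player and shows a floating prompt.
; Pickup clears its list entry except hex index; a swap stores the player's old equipment there and spawns it in place before self-destructing.
; Child hooks define passive and shelter abilities, the latter modifying target hexes or acting globally when no pattern exists.
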(event OnComponentBeginOverlap(PickupOverlap)
  (params (OverlappedComponent :type Primitive%20Component%20Object%20Reference) (OtherActor :type Actor%20Object%20Reference) (OtherComp :type Primitive%20Component%20Object%20Reference) (OtherBodyIndex :type Integer) (bFromSweep :type Boolean) (SweepResult :type Hit%20Result%20Structure%20%28by%20ref%29))
  ;[1 1 1] Pickup setup
  (bind _asbp_player (Utilities|Casting|CastToBP_Player OtherActor))
  (bind _output_get (Variables|Default|SetPlayerRef _asbp_player))
  (Variables|/Game/Characters/BP_Player.BP_Player_C|SetOverlappedActorRef _output_get self)
  ;[1 1 1] Help text display
  (bind _index (Default|DisplayText (Variables|Default|GetFloatingTextManager) (Utilities|Struct|MakeFloatingTextParameters "NewEnumerator1" (Variables|Default|GetDefaultSceneRoot) false 1.5e+02 3e+02 1e+02 "(X=-1.000000,Y=-1.000000)") (Utilities|Array|MakeArray (Utilities|String|ToString(Text) (Utilities|Text|MakeLiteralText "Press <E> to pickup")))))
  (Variables|Default|SetHelpTextIndex _index))

(event OnComponentEndOverlap(PickupOverlap)
  (params (OverlappedComponent :type Primitive%20Component%20Object%20Reference) (OtherActor :type Actor%20Object%20Reference) (OtherComp :type Primitive%20Component%20Object%20Reference) (OtherBodyIndex :type Integer))
  ;[1 1 1] Pickup setup
  (bind _asbp_player (Utilities|Casting|CastToBP_Player OtherActor))
  (Variables|/Game/Characters/BP_Player.BP_Player_C|SetOverlappedActorRef _asbp_player (Utilities|Null))
  ;[1 1 1] Help text display
  (Default|FadeOutText (Variables|Default|GetFloatingTextManager) (Variables|Default|GetHelpTextIndex))
  (Variables|Default|SetHelpTextIndex -1))

(event Custom|NotifyItemAdded
  (params (Type :type ItemType%20Enum))
  ;[1 1 1] For override by children
)

(event EventGenericInteractwithSomething
  (bind _playerref (Variables|Default|GetPlayerRef))
  (bind _currentequipment (Variables|/Game/Characters/BP_Player.BP_Player_C|GetCurrentEquipment _playerref))
  ;[1 1 1] Pickup setup
  (if (Utilities|IsValidClass (.equipClass (Utilities|Struct|BreakEquipInfo _currentequipment)))
    (CallFunction|CallPlayerforSwitch _currentequipment)
    (else
      (CallFunction|CallPlayerforPickup)))
  ;[1 1 1] Help text display
  (Default|DestroyText (Variables|Default|GetFloatingTextManager) (Variables|Default|GetHelpTextIndex))
  (Actor|DestroyActor))

(event EventBeginPlay
  (bind _asmultivrs_game_instance (Utilities|Casting|CastToMultivrsGameInstance (Game|GetGameInstance)))
  (bind _output_get (Variables|Default|SetGameInstanceRef _asmultivrs_game_instance))
  (Variables|Default|SetTooltipText (.equipName (Utilities|Struct|BreakEquipInfo (.equipmentinfo (Utilities|Array|Get(acopy) (Variables|/Game/Foundation/MultivrsGameInstance.MultivrsGameInstance_C|GetObservedEquipments _output_get) (Variables|Default|GetObservedEquipIndex)))))))

(fn ConstructionScript
  (Variables|Default|SetPickupRadius (Utilities|CONSTPickupEquipmentRadius))
  (Variables|Default|SetTooltipRadius (Utilities|CONSTTooltipEquipmentRadius))
  (|CallParentFunction))

(fn CallPlayerforSwitch
  (params (EquipInfo :type Equip%20Info%20Structure))
  ;[1 1 1] Store current for switch
  (LocalVariables|Set_EquipInfo EquipInfo)
  (LocalVariables|Set_HexIndex (.observedhexindex (Utilities|Array|Get(acopy) (Variables|/Game/Foundation/MultivrsGameInstance.MultivrsGameInstance_C|GetObservedEquipments (Variables|Default|GetGameInstanceRef)) (Variables|Default|GetObservedEquipIndex))))
  (Utilities|FlowControl|Sequence
    (:then_0
      ;[1 1 1] Call pickup
      (CallFunction|CallPlayerforPickup))
    (:then_1
      ;[1 1 1] Set equip infos in observed list
      (Utilities|Array|SetArrayElem (Variables|/Game/Foundation/MultivrsGameInstance.MultivrsGameInstance_C|GetObservedEquipments (Variables|Default|GetGameInstanceRef)) (Variables|Default|GetObservedEquipIndex) (Utilities|Struct|MakeEquipmentContainer (LocalVariables|Get_EquipInfo) (LocalVariables|Get_HexIndex))))
    (:then_2
      ;[1 1 1] Spawn new equipment at same location
      (bind _returnvalue (Game|SpawnActorfromClass (.equipClass (Utilities|Struct|BreakEquipInfo (LocalVariables|Get_EquipInfo))) (Transformation|GetActorTransform) "Undefined" 0 0))
      (bind _asbp_equipment (Utilities|Casting|CastToBP_Equipment _returnvalue))
      (Variables|BP_Equipment_C|SetObservedEquipIndex _asbp_equipment (Variables|Default|GetObservedEquipIndex)))))

(fn CallPlayerforPickup
  (bind _observedequipindex (Variables|Default|GetObservedEquipIndex))
  (bind _gameinstanceref (Variables|Default|GetGameInstanceRef))
  (bind _observedequipments (Variables|/Game/Foundation/MultivrsGameInstance.MultivrsGameInstance_C|GetObservedEquipments _gameinstanceref))
  (bind _item (Utilities|Array|Get(acopy) _observedequipments _observedequipindex))
  (Default|PickupEquipment (Variables|Default|GetPlayerRef) (.equipmentinfo _item))
  (Utilities|Array|SetArrayElem _observedequipments _observedequipindex (Utilities|Struct|MakeEquipmentContainer "(equipClass=None,chanceWeight=0.000000,equipName=\"\",equipDescription=\"\",equipTexture=None,equipAbilityName=\"\",equipAbilityDescription=\"\",equipAbilityTime=0.000000)" (.observedhexindex _item))))

(fn EnablePassiveAbility)

(fn DisablePassiveAbility)

(fn ActivateShelterAbility
  (params (TargetCoord :type Array%20of%20Hex%20Cube%20Coordinates%20Structures))
  (if (> (Utilities|String|Len (.equipAbilityHexPattern (Utilities|Struct|BreakEquipInfo (.equipmentinfo (Utilities|Array|Get(acopy) (Variables|/Game/Foundation/MultivrsGameInstance.MultivrsGameInstance_C|GetObservedEquipments (Variables|Default|GetGameInstanceRef)) (Variables|Default|GetObservedEquipIndex)))))) 0)
    (for _array_element TargetCoord
      (bind (_outtype _outmodifier) (CallFunction|HexShelterAbilityEffect (.Container (Default|GetHexContainerfromCoord (Variables|Default|GetGameInstanceRef) _array_element))))
      (Default|ModifyHex (Variables|Default|GetGameInstanceRef) (.Index (Default|GetHexContainerfromCoord (Variables|Default|GetGameInstanceRef) _array_element)) _outtype _outmodifier))
    (else
      (CallFunction|GlobalShelterAbilityEffect))))

(fn HexShelterAbilityEffect
  (params (InContainer :type Hex%20Container%20Structure))
  (bind (_coordinates _hextype _universedbindex _isvisible _modifier) (Utilities|Struct|BreakHexContainer InContainer))
  (return _hextype _modifier))

(fn GlobalShelterAbilityEffect)