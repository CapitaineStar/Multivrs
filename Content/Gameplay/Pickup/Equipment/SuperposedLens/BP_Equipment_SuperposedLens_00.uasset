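; Superposed Lens equipment Blueprint that can be enabled or disabled and tops up the player's spotter counts when items are added.
; Enable and disable events only toggle an IsEnabled flag, which the item notification does not check.
; NotifyItemAdded casts player 0 to BP_Player and increments its Location or Momentum Spotter count by item type, capped at that type's maximum.
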(event Custom|EnableAbility_1
  (Variables|Default|SetIsEnabled true))

(event Custom|DisableAbility_1
  (Variables|Default|SetIsEnabled false))

(event EventNotifyItemAdded
  (params (Type :type ItemType%20Enum))
  (bind _asbp_player (Utilities|Casting|CastToBP_Player (Game|GetPlayerCharacter 0)))
  ;[1 1 1] Check if full and increment if not
  (switch Utilities|FlowControl|Switch|SwitchonItemType Type
    (:NewEnumerator0
      (if (< (Variables|/Game/Characters/BP_Player.BP_Player_C|GetLocationSpotterNb _asbp_player) (Variables|/Game/Characters/BP_Player.BP_Player_C|GetLocationSpotterMax _asbp_player))
        (Math|Integer|IncrementInt (Variables|/Game/Characters/BP_Player.BP_Player_C|GetLocationSpotterNb _asbp_player))))
    (:NewEnumerator1
      (if (< (Variables|/Game/Characters/BP_Player.BP_Player_C|GetMomentumSpotterNb _asbp_player) (Variables|/Game/Characters/BP_Player.BP_Player_C|GetMomentumSpotterMax _asbp_player))
        (Math|Integer|IncrementInt (Variables|/Game/Characters/BP_Player.BP_Player_C|GetMomentumSpotterNb _asbp_player))))))

(fn ConstructionScript
  (|CallParentFunction))