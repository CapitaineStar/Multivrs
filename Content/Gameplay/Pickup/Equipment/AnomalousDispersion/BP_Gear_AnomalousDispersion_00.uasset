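; Anomalous Dispersion equipment gear that grants a passive movement boost and alters a hex shelter's wind.
; Enabling the passive multiplies the player character's walk speed and jump velocity by one shared multiplier, and disabling divides them back rather than restoring cached values.
; Its shelter effect returns the hex type unchanged and a modifier with only wind speed scaled, passing the other fields through.
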(event EventBeginPlay)

(event Collision|EventActorBeginOverlap
  (params (OtherActor :type Actor%20Object%20Reference)))

(event EventTick
  (params (DeltaSeconds :type Float%20%28single-precision%29)))

(event EventEnablePassiveAbility
  (bind _returnvalue (Game|GetPlayerCharacter 0))
  (bind _charactermovement (Variables|/Script/Engine.Character|GetCharacterMovement _returnvalue))
  (Variables|/Script/Engine.CharacterMovementComponent|SetMaxWalkSpeed _charactermovement (* (Variables|/Script/Engine.CharacterMovementComponent|GetMaxWalkSpeed _charactermovement) (Variables|Default|GetWalkSpeedMultiplier)))
  (Variables|/Script/Engine.CharacterMovementComponent|SetJumpZVelocity _charactermovement (* (Variables|/Script/Engine.CharacterMovementComponent|GetJumpZVelocity _charactermovement) (Variables|Default|GetWalkSpeedMultiplier))))

(event EventDisablePassiveAbility
  (bind _returnvalue (Game|GetPlayerCharacter 0))
  (bind _charactermovement (Variables|/Script/Engine.Character|GetCharacterMovement _returnvalue))
  (Variables|/Script/Engine.CharacterMovementComponent|SetMaxWalkSpeed _charactermovement (/ (Variables|/Script/Engine.CharacterMovementComponent|GetMaxWalkSpeed _charactermovement) (Variables|Default|GetWalkSpeedMultiplier)))
  (Variables|/Script/Engine.CharacterMovementComponent|SetJumpZVelocity _charactermovement (/ (Variables|/Script/Engine.CharacterMovementComponent|GetJumpZVelocity _charactermovement) (Variables|Default|GetWalkSpeedMultiplier))))

(fn ConstructionScript
  (|CallParentFunction))

(fn HexShelterAbilityEffect
  (params (InContainer :type Hex%20Container%20Structure))
  (bind (_coordinates _hextype _universedbindex _isvisible _modifier) (Utilities|Struct|BreakHexContainer InContainer))
  (bind (_windspeed _entropyamount _spottersamount _trapsamount _preylure) (Utilities|Struct|BreakHexModifier _modifier))
  (return _hextype (Utilities|Struct|MakeHexModifier (* _windspeed (Variables|Default|GetWindSpeedMultiplier)) _entropyamount _spottersamount _trapsamount _preylure)))