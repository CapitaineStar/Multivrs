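; BP_SplinePath is an actor that wraps a spline component as a path that other code can grow and shrink.
; Construction clears all default points, so the path starts empty.
; ExtendSpline appends a world-space point and ShortenSpline removes the first, so points behave as a first-in, first-out queue.
; GetMaxDistance returns the distance to the last point; the event graph has no active logic.
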(event EventBeginPlay)

(event Collision|EventActorBeginOverlap
  (params (OtherActor :type Actor%20Object%20Reference)))

(event EventTick
  (params (DeltaSeconds :type Float%20%28single-precision%29)))

(fn ConstructionScript
  (Spline|ClearSplinePoints (Variables|Default|GetSpline) true))

(fn ExtendSpline
  (params (PointLocation :type Vector))
  (Spline|AddSplinePoint (Variables|Default|GetSpline) PointLocation "World" true))

(fn ShortenSpline
  (Spline|RemoveSplinePoint (Variables|Default|GetSpline) 0 true))

(fn GetMaxDistance
  (bind _spline (Variables|Default|GetSpline))
  (return (Spline|GetDistanceAlongSplineatSplinePoint _spline (- (Spline|GetNumberOfSplinePoints _spline) 1))))