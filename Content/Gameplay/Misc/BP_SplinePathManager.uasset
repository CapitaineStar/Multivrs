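; BP_SplinePathManager spawns and manages spline paths for the prey and the player on the hex-tile world.
; Tick moves a prey location component along its spline at difficulty-based speed.
; A timer extends that spline via an EQS query from its end point, unspawning prey whose projected coordinate leaves loading range.
; Another timer records player movement as a point-capped trail and makes hexes visible as it extends.
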(event Custom|RunEnvQuery
  ;[1 1 1] Environment Query
  (bind _returnvalue (AI|EQS|RunEQSQuery (Variables|Default|GetQueryTemplate) (Variables|Default|GetActivePreyEndPoint) "RandomBest25Pct"))
  (EventDispatchers|BindEventtoOnQueryFinishedEvent _returnvalue (delegate Custom|OnQueryFinished)))

(event Custom|OnQueryFinished
  (params (QueryInstance :type Env%20Query%20Instance%20Blueprint%20Wrapper%20Object%20Reference) (QueryStatus :type EEnvQueryStatus%20Enum))
  (bind _returnvalue (Class|EnvQueryInstanceBlueprintWrapper|GetResultsasLocations QueryInstance))
  ;[1 1 1] Environment Query
  (if (== (Utilities|Array|Length _returnvalue) 1)
    (CallFunction|ExtendPath (Utilities|Array|Get(acopy) _returnvalue) (Variables|Prey|GetActivePreyPathIndex) (Variables|Default|GetActivePreyEndPoint))
    (else
      (Development|PrintString "Warning, query not returning one result"))))

(event Custom|StartManagePreyPath
  ;[1 1 1] ManagePreyPath timer
  (bind _returnvalue (Utilities|Time|SetTimerbyFunctionName 0 "ManagePreyPath" 1.0 true))
  (Variables|Prey|SetPreyPathTimerHandle _returnvalue))

(event Custom|StopManagePreyPath
  ;[1 1 1] ManagePreyPath timer
  (if (Utilities|Time|IsValidTimerHandle (Variables|Prey|GetPreyPathTimerHandle))
    (Utilities|Time|ClearandInvalidateTimerbyHandle (Variables|Prey|GetPreyPathTimerHandle))))

(event Custom|StartManagePlayerPath
  ;[1 1 1] ManagePlayerPath timer
  (bind _returnvalue (Utilities|Time|SetTimerbyFunctionName 0 "ManagePlayerPath" 0.5 true))
  (Variables|Player|SetPlayerPathTimerHandle _returnvalue))

(event Custom|StopManagerPlayerPath
  ;[1 1 1] ManagePlayerPath timer
  (if (Utilities|Time|IsValidTimerHandle (Variables|Player|GetPlayerPathTimerHandle))
    (Utilities|Time|ClearandInvalidateTimerbyHandle (Variables|Player|GetPlayerPathTimerHandle))))

(event EventBeginPlay
  (bind _asmultivrs_game_instance (Utilities|Casting|CastToMultivrsGameInstance (Game|GetGameInstance)))
  (bind _output_get (Variables|References|SetGameInstanceRef _asmultivrs_game_instance))
  (bind _asmultivrs_game_mode (Utilities|Casting|CastToMultivrsGameMode (Game|GetGameMode)))
  (Variables|References|SetGameModeRef _asmultivrs_game_mode)
  (Variables|Default|SetCurrentBiome (Default|GetCurrentBiome _output_get))
  (Variables|Prey|SetPreyMoveSpeed (.Prey_NearMoveSpeed (Utilities|Struct|BreakGameVariables (Default|GetCurrentDifficulty _output_get)))))

(event EventTick
  (params (DeltaSeconds :type Float%20%28single-precision%29))
  (if (Variables|Prey|GetIsPreyMoving)
    (Prey|MovePreyLocation DeltaSeconds)))

(fn ConstructionScript)

(fn MovePreyLocation
  (params (DeltaTime :type Float%20%28single-precision%29))
  (bind _spline (Utilities|ActivePreySpline))
  (bind _preylocation (Variables|Default|GetPreyLocation))
  (bind _output_get (Variables|Prey|SetPreyDistance (+ (Variables|Prey|GetPreyDistance) (* DeltaTime (Variables|Prey|GetPreyMoveSpeed)))))
  (Transformation|SetWorldLocation _preylocation (Spline|GetLocationatDistanceAlongSpline _spline _output_get "World") false false)
  (Transformation|SetWorldRotation _preylocation (Spline|GetRotationatDistanceAlongSpline _spline _output_get "World") false false))

(fn ManagePreyPath
  (bind _spline (Utilities|ActivePreySpline))
  (bind _returnvalue (Spline|GetNumberOfSplinePoints _spline))
  (bind _returnvalue_2 (- _returnvalue 1))
  (Utilities|FlowControl|Sequence
    (:then_0
      ;[1 1 1] Check if on second to last segment
      (if (not (<= _returnvalue_2 (+ (Math|Float|Round (* _returnvalue_2 (Class|SplineComponent|GetInputKeyatDistanceAlongSpline _spline (Variables|Prey|GetPreyDistance)))) 1)))
        (return)))
    (:then_1
      (bind _ispreyinrange (Prey|LookAhead (Transformation|GetActorLocation (Variables|References|GetPreyRef))))
      (if (not _ispreyinrange)
        (return)))
    (:then_2
      (CallFunction|RunEnvQuery)
      (return))))

(fn LookAhead
  (params (Location :type Vector))
  (LocalVariables|Set_CurrentLocation Location)
  (Utilities|IsValid (Variables|References|GetPreyRef)
    (:Is%20Valid
      (Utilities|FlowControl|Sequence
        (:then_0
          ;[1 1 1] Calculate probable next Hex coord
          (LocalVariables|Set_ProbableNextCoord (CallFunction|ToHexCoord(WorldPosition) (* (+ (* (Math|Vector|RotateVector "1.000000, 0, 0" (Math|Rotator|MakeRotator 0.0 0.0 (Variables|/Game/Foundation/MultivrsGameMode.MultivrsGameMode_C|GetPreyMomentum (Variables|References|GetGameModeRef)))) 2e+03) (LocalVariables|Get_CurrentLocation)) (.HexTileScale (Utilities|Struct|BreakBiomeDescription (Variables|Default|GetCurrentBiome)))))))
        (:then_1
          ;[1 1 1] Check if will be in loading range
          (if (> (CallFunction|Distance(HexCoord) (Variables|/Game/Foundation/MultivrsGameMode.MultivrsGameMode_C|GetCurrentCoord (Variables|References|GetGameModeRef)) (LocalVariables|Get_ProbableNextCoord)) (.LoadingRange (Utilities|Struct|BreakBiomeDescription (Variables|Default|GetCurrentBiome))))
            ;[1 1 1] Unspawn if true
            (Default|UnSpawnPrey (Variables|References|GetGameModeRef) (LocalVariables|Get_ProbableNextCoord))
            (CallFunction|StopManagePreyPath)
            (Variables|Prey|SetIsPreyMoving false)
            (LocalVariables|Set_IsPreyInRange false)
            (else
              (LocalVariables|Set_IsPreyInRange true))))
        (:then_2
          (return (LocalVariables|Get_IsPreyInRange)))))
    (:Is%20Not%20Valid
      (return (LocalVariables|Get_IsPreyInRange)))))

(fn CreateNewPath
  (params (StartLocation :type Vector) (IsForPrey :type Boolean))
  (LocalVariables|Set_Location StartLocation)
  (LocalVariables|Set_IsForPrey IsForPrey)
  (Utilities|FlowControl|Sequence
    (:then_0
      ;[1 1 1] Spawn new SplinePath actor
      (bind _returnvalue (Game|SpawnActorfromClass "/Game/Gameplay/Misc/BP_SplinePath.BP_SplinePath_C" (Math|Conversions|ToTransform(Vector) (LocalVariables|Get_Location)) "Undefined" self 0))
      (Transformation|AttachActorToActor _returnvalue self "None" "KeepWorld" "KeepWorld" "KeepWorld" true)
      (bind _returnvalue_2 (Utilities|Array|Add (Variables|Default|GetPathsArray) _returnvalue))
      (LocalVariables|Set_PathIndex _returnvalue_2))
    (:then_1
      ;[1 1 1] Place first spline point
      (if (LocalVariables|Get_IsForPrey)
        (CallFunction|ExtendPath (LocalVariables|Get_Location) (LocalVariables|Get_PathIndex) (Variables|Default|GetActivePreyEndPoint))
        (Prey|SetupPreyPath true (LocalVariables|Get_PathIndex) (LocalVariables|Get_Location))
        (else
          (CallFunction|ExtendPath (LocalVariables|Get_Location) (LocalVariables|Get_PathIndex) (Variables|Default|GetActivePlayerEndPoint)))))
    (:then_2
      (return (LocalVariables|Get_PathIndex)))))

(fn ExtendPath
  (params (PointLocation :type Vector) (PathIndex :type Integer) (EndPointComponent :type Static%20Mesh%20Component%20Object%20Reference))
  (Default|ExtendSpline (Utilities|Array|Get(acopy) (Variables|Default|GetPathsArray) PathIndex) PointLocation)
  (Transformation|SetWorldLocation EndPointComponent PointLocation false true))

(fn ManagePlayerPath
  (Variables|References|GetPlayerRef
    (:then
      (Utilities|FlowControl|Sequence
        (:then_0
          ;[1 1 1] Extend path if player moved beyond threshold
          (if (>= (Math|Vector|VectorLength (- (Transformation|GetActorLocation (Variables|References|GetPlayerRef)) (Transformation|GetWorldLocation (Variables|Default|GetActivePlayerEndPoint)))) (Variables|Player|GetPlayerPathPointThreshold))
            (CallFunction|ExtendPath (Transformation|GetActorLocation (Variables|References|GetPlayerRef)) (Variables|Player|GetActivePlayerPathIndex) (Variables|Default|GetActivePlayerEndPoint))
            (LocalVariables|Set_IsExtended true)))
        (:then_1
          ;[1 1 1] Shorten path if reach map number of spline points
          (if (> (Spline|GetNumberOfSplinePoints (Utilities|ActivePlayerSpline)) (Variables|Player|GetPlayerMaxPathPoints))
            (CallFunction|ShortenPath (Variables|Player|GetActivePlayerPathIndex))))
        (:then_2
          (if (LocalVariables|Get_IsExtended)
            (Default|SetHexCoordVisibility (Variables|References|GetGameInstanceRef) (CallFunction|ToHexCoord(WorldPosition) (Transformation|GetActorLocation (Variables|References|GetPlayerRef))) true)))))
    (:else)))

(fn ShortenPath
  (params (PathIndex :type Integer))
  (Default|ShortenSpline (Utilities|Array|Get(acopy) (Variables|Default|GetPathsArray) PathIndex)))

(fn GetActivePlayerSpline
  (return (Utilities|Array|Get(acopy) (Variables|Default|GetPathsArray) (Variables|Player|GetActivePlayerPathIndex))))

(fn SetupPreyPath
  (params (IsPreyMoving :type Boolean) (PathIndex :type Integer) (StartLocation :type Vector))
  (Variables|Prey|SetIsPreyMoving IsPreyMoving)
  (Variables|Prey|SetActivePreyPathIndex PathIndex)
  (Variables|Prey|SetPreyDistance -1e+03)
  (Transformation|SetWorldLocation (Variables|Default|GetPreyLocation) StartLocation false false))