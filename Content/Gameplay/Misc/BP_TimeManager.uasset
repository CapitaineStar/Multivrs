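; Time manager actor that fast-forwards the game by a requested time jump, ramping global time dilation up to a top speed and back down.
; FastForward splits the jump into ease-in, cruise and ease-out phases using the ease curve's analytic integral, shortening the ramps for small jumps.
; Tick steps through the phases, setting the actor's custom dilation to the inverse of global dilation so its own timing stays in real time.
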(event EventBeginPlay
  (bind _asmultivrs_game_mode (Utilities|Casting|CastToMultivrsGameMode (Game|GetGameMode)))
  (Variables|Default|SetGameModeRef _asmultivrs_game_mode)
  ;[1 1 1] Get Total time if using full range of Ease In/Out curve
  (Variables|Default|SetFFwdEaseTotalTime (* (Math|Float|MapRangeClamped (Utilities|FFwdEaseinOutIntegral (Variables|Default|GetFFwdEaseInOutDuration)) 0.0 1.0 1.0 (Variables|Default|GetFFwdTopSpeed)) 2.0)))

(event EventTick
  (params (DeltaSeconds :type Float%20%28single-precision%29))
  (if (Variables|Default|GetIsFFwding)
    (CallFunction|FastForwardStep DeltaSeconds)))

(fn ConstructionScript)

(fn GetFFwdTimeDuration
  (params (TimeJump :type Float%20%28single-precision%29))
  (LocalVariables|Set_TimeJump TimeJump)
  (Utilities|FlowControl|Sequence
    (:then_0
      ;[1 1 1] Check if time is left after Ease In/Out and set cruising time
      (if (> (LocalVariables|Get_TimeJump) (Variables|Default|GetFFwdEaseTotalTime))
        (LocalVariables|Set_TimeCruising (/ (- (LocalVariables|Get_TimeJump) (Variables|Default|GetFFwdEaseTotalTime)) (Variables|Default|GetFFwdTopSpeed)))
        (LocalVariables|Set_TimeAccel+Decel (* (Variables|Default|GetFFwdEaseInOutDuration) 2.0))
        (else
          ;[1 1 1] Else, reduce Ease In/Out duration
          (LocalVariables|Set_TimeCruising 0.0)
          (LocalVariables|Set_TimeAccel+Decel (* (/ (LocalVariables|Get_TimeJump) (Variables|Default|GetFFwdEaseTotalTime)) (* (Variables|Default|GetFFwdEaseInOutDuration) 2.0))))))
    (:then_1
      (return (LocalVariables|Get_TimeAccel+Decel) (LocalVariables|Get_TimeCruising)))))

(fn FastForward
  (params (TimeJump :type Float%20%28single-precision%29))
  (if (> TimeJump 0.0)
    (bind (_timeaccel_decel _timecruising) (CallFunction|GetFFwdTimeDuration TimeJump))
    (Variables|Default|SetCurrentFFwdEaseIn (/ _timeaccel_decel 2.0))
    (Variables|Default|SetCurrentFFwdEaseOut (/ _timeaccel_decel 2.0))
    (Variables|Default|SetCurrentFFwdEaseMult (/ (/ _timeaccel_decel 2.0) (Variables|Default|GetFFwdEaseInOutDuration)))
    (Variables|Default|SetCurrentFFwdCruising _timecruising)
    (Variables|Default|SetIsFFwding true)))

(fn FastForwardStep
  (params (DeltaTime :type Float%20%28single-precision%29))
  (LocalVariables|Set_DeltaTime DeltaTime)
  (Utilities|FlowControl|Sequence
    (:then_0
      (if (> (Variables|Default|GetCurrentFFwdEaseIn) 0.0)
        ;[1 1 1] EaseIn
        (bind _output_get (Variables|Default|SetCurrentFFwdEaseIn (- (Variables|Default|GetCurrentFFwdEaseIn) (LocalVariables|Get_DeltaTime))))
        (LocalVariables|Set_TimeDilation (Utilities|FFwdEaseinOut (/ (- 1.0 _output_get) (Variables|Default|GetCurrentFFwdEaseMult))))
        (elif (> (Variables|Default|GetCurrentFFwdCruising) 0.0)
          ;[1 1 1] Cruising
          (Variables|Default|SetCurrentFFwdCruising (- (Variables|Default|GetCurrentFFwdCruising) (LocalVariables|Get_DeltaTime)))
          (LocalVariables|Set_TimeDilation (Variables|Default|GetFFwdTopSpeed))
          (elif (> (Variables|Default|GetCurrentFFwdEaseOut) 0.0)
            ;[1 1 1] EaseIn
            (bind _output_get_2 (Variables|Default|SetCurrentFFwdEaseOut (- (Variables|Default|GetCurrentFFwdEaseOut) (LocalVariables|Get_DeltaTime))))
            (LocalVariables|Set_TimeDilation (Utilities|FFwdEaseinOut (/ _output_get_2 (Variables|Default|GetCurrentFFwdEaseMult))))
            (else
              (Variables|Default|SetIsFFwding false))))))
    (:then_1
      (if (Variables|Default|GetIsFFwding)
        (Utilities|Time|SetGlobalTimeDilation (LocalVariables|Get_TimeDilation))
        (Variables|Default|SetCustomTimeDilation (/ 1.0 (LocalVariables|Get_TimeDilation)))
        (else
          (Utilities|Time|SetGlobalTimeDilation 1.0)
          (Variables|Default|SetCustomTimeDilation 1.0))))))